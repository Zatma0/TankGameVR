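; BP_EnemySpawner runs the timed enemy wave loop for the tank game, starting after a short delay at BeginPlay.
; A timer ends each wave, then WaveOver increments the count, scales wave length and break time within clamps, and starts the next wave.
; EnemyUnlock raises max base spawn rates for armored cars, tanks and anti-tanks at different wave intervals.
; SpawnEnemies is called each wave but is empty here.
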(event `SpawnEnemies`)

(event `self.ReceiveBeginPlay`
  ; To Keep Event BeginPlay Clean
  (`KismetSystemLibrary.Delay` 10.0)
  (`self.WaveBeginning`)
  (`self.SpawnEnemies`))

(event `WaveBeginning`
  (bind _returnvalue (`KismetSystemLibrary.K2_SetTimerDelegate` (delegate `WaveOver`) (`self.WaveTimer`)))
  (set `self.TimerHandle` _returnvalue))

(event `WaveOver`
  ;[0.3559 0.3559 0.3559 0.5] Calculating New Wave Count & Timer Time - Call Spawn Enemies
  (bind _result (`/Engine/EditorBlueprintResources/StandardMacros.IncrementInt` (`self.WaveCount`))
    (:`  `
      (bind _output_get (set `self.WaveCount` _result))
      (`self.EnemyUnlock`)
      (set `self.WaveTimer` (`KismetMathLibrary.Conv_IntToDouble` (`KismetMathLibrary.Clamp` (* _output_get 30) 30 600)))
      (`KismetSystemLibrary.Delay` (`KismetMathLibrary.Conv_IntToDouble` (`KismetMathLibrary.Clamp` (* (`self.WaveCount`) 5) 5 120)))
      (`self.WaveBeginning`)
      (`self.SpawnEnemies`))))

(event `EnemyUnlock`
  ; Adjusting the Spawn Rates of Enemy Types
  (`|ExecutionSequence`
    (:`then_0`
      (if (== (mod (`self.WaveCount`) 1) 0)
        (bind _result (`/Engine/EditorBlueprintResources/StandardMacros.IncrementInt` (`self.MaxArmoredCar_SpawnRateBase`))
          (:`  `
            (set `self.MaxArmoredCar_SpawnRateBase` _result)))))
    (:`then_1`
      (if (== (mod (`self.WaveCount`) 3) 0)
        (bind _result_2 (`/Engine/EditorBlueprintResources/StandardMacros.IncrementInt` (`self.MaxTank_SpawnRateBase`))
          (:`  `
            (set `self.MaxTank_SpawnRateBase` _result_2)))))
    (:`then_2`
      (if (== (mod (`self.WaveCount`) 7) 0)
        (bind _result_3 (`/Engine/EditorBlueprintResources/StandardMacros.IncrementInt` (`self.MaxAntiTank_SpawnRateBase`))
          (:`  `
            (set `self.MaxAntiTank_SpawnRateBase` _result_3)))))))

(fn `UserConstructionScript`)