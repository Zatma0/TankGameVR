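; BP_EnemyBase is the base enemy Blueprint for the tank game, giving each enemy its visual model.
; On BeginPlay it runs SetEnemyMesh, which switches on SpawnedEnemyType (Tank, Armored Car or Anti Tank) and assigns the static mesh from Features.E_Model.
; All three branches make the same assignment, so the model depends only on the Features data.
; The construction script is empty.
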(event `self.ReceiveBeginPlay`
  (`self.SetEnemyMesh`))

(fn `SetEnemyMesh`
  (bind (_features_e_enemytype _features_e_hp _features_e_damage _features_e_speed _features_e_range _features_e_model) (break `/Game/TankGame/Ugurkan/BPs/Gameplay/EnemyInfos/S_EnemyFeatures` (`self.Features`)))
  (switch `/Game/TankGame/Ugurkan/BPs/Gameplay/EnemyInfos/E_EnemyTypes` (`self.SpawnedEnemyType`)
    (:`NewEnumerator0`
      (`StaticMeshComponent.SetStaticMesh` (`self.StaticMesh`) _features_e_model))
    (:`NewEnumerator1`
      (`StaticMeshComponent.SetStaticMesh` (`self.StaticMesh`) _features_e_model))
    (:`NewEnumerator2`
      (`StaticMeshComponent.SetStaticMesh` (`self.StaticMesh`) _features_e_model))))

(fn `UserConstructionScript`)