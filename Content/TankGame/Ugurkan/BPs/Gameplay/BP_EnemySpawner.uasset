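; Enemy wave spawner that runs timed waves of armored cars, tanks and anti-tank guns.
; A wave timer and break delay advance the count, scaling spawn weights, wave length, enemy count and spawn pace through game phases.
; A delayed self-calling event spawns weighted picks one by one, using DataTable stats and hidden transforms from the director.
; It also shows the wave HUD and reports wave number and countdown to the director.
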(event `SpawnEnemies`
  ;[0.7205 0 0.01285 0.5] SpawnEnemies Custom Event
  (set `self.SpawnedThisWave` 0)
  (`self.SpawnNextEnemy`))

(event `SpawnNextEnemy`
  ; One enemy at a time until MaxSpawnedEnemyValue: weighted type, a spot the player is not looking at, then wait Min-Max delay.
  ;;[0.7205 0 0.01285 0.5] SpawnEnemies Custom Event
  (if (< (`self.SpawnedThisWave`) (`self.MaxSpawnedEnemyValue`))
    (bind (_enemytype _rowname) (`self.PickEnemyType`))
    (bind _returnvalue (`|GetDataTableRow` "/Game/TankGame/Ugurkan/BPs/Gameplay/EnemyInfos/DT_EnemyFeatures.DT_EnemyFeatures" _rowname)
      (:`then`
        (bind (_boutofsight _returnvalue_2) (`TankArenaDirector.GetHiddenSpawnTransformByIndex` (`TankArenaDirector.GetDirector`) (`KismetMathLibrary.Conv_ByteToInt` _enemytype)))
        (bind (_e_enemytype _e_hp _e_damage _e_speed _e_range _e_model) (break `/Game/TankGame/Ugurkan/BPs/Gameplay/EnemyInfos/S_EnemyFeatures` _returnvalue))
        (bind _returnvalue_3 (`|SpawnActorFromClass` "/Game/TankGame/Ugurkan/BPs/Gameplay/BP_EnemyBase.BP_EnemyBase_C" (`KismetMathLibrary.MakeTransform` (.location _returnvalue_2) (.rotation _returnvalue_2) (.scale _returnvalue_2)) "AdjustIfPossibleButAlwaysSpawn" "MultiplyWithRoot" null (make `/Game/TankGame/Ugurkan/BPs/Gameplay/EnemyInfos/S_EnemyFeatures` _e_enemytype _e_hp _e_damage _e_speed _e_range _e_model) null))
        (set `/Game/TankGame/Ugurkan/BPs/Gameplay/BP_EnemyBase.SpawnedEnemyType` _enemytype _returnvalue_3))
      (:`RowNotFound`
        (`KismetSystemLibrary.PrintString` "Row Unfound")))
    (`/Engine/EditorBlueprintResources/StandardMacros.IncrementInt` (`self.SpawnedThisWave`)
      (:`  `
        (`KismetSystemLibrary.Delay` (`KismetMathLibrary.RandomFloatInRange` (`self.EnemyMinSpawnDelay`) (`self.EnemyMaxSpawnDelay`)))
        (`self.SpawnNextEnemy`)))))

(event `self.ReceiveBeginPlay`
  ; One enemy at a time until MaxSpawnedEnemyValue: weighted type, a spot the player is not looking at, then wait Min-Max delay.
  ;; To Keep Event BeginPlay Clean
  ;; Wave panel on the screen; the director (cockpit display) learns the waves come from here.
  ;; First wave size is worked out before it starts.
  (`TankWaveHudWidget.ShowWaveHud` null)
  (`TankArenaDirector.SetExternalWave` (`TankArenaDirector.GetDirector`) 0 10.0)
  ;; Cockpit display and wave panel: which wave, and how long until the next one.
  (`self.MaxEnemySpawnCalculation`)
  (`KismetSystemLibrary.Delay` 10.0)
  (`self.WaveBeginning`)
  (`self.SpawnEnemies`))

(event `WaveBeginning`
  ; Wave panel on the screen; the director (cockpit display) learns the waves come from here.
  ; First wave size is worked out before it starts.
  (bind _returnvalue (`KismetSystemLibrary.K2_SetTimerDelegate` (delegate `WaveOver`) (`self.WaveTimer`)))
  (set `self.TimerHandle` _returnvalue)
  ; Cockpit display and wave panel: which wave, and how long until the next one.
  (`TankArenaDirector.SetExternalWave` (`TankArenaDirector.GetDirector`) (`self.WaveCount`) (`self.GetSecondsToNextWave`)))

(event `WaveOver`
  ;[0.1288 0.3559 0 0.5] Calculating New Wave Count & Timer Time - Call Spawn Enemies
  (bind _result (`/Engine/EditorBlueprintResources/StandardMacros.IncrementInt` (`self.WaveCount`))
    (:`  `
      (bind _output_get (set `self.WaveCount` _result))
      (`self.EnemyWaveAdjustment`)
      ;; Cockpit display and wave panel: which wave, and how long until the next one.
      (set `self.WaveTimer` (`KismetMathLibrary.Conv_IntToDouble` (`KismetMathLibrary.Clamp` (* _output_get 30) 30 600)))
      (`KismetSystemLibrary.Delay` (`KismetMathLibrary.Conv_IntToDouble` (`KismetMathLibrary.Clamp` (* (`self.WaveCount`) 5) 5 120)))
      (`self.WaveBeginning`)
      (`KismetSystemLibrary.Delay` 3.0)
      (`self.SpawnEnemies`))))

(event `EnemyWaveAdjustment`
  ;[0.00044 0.08868 0.15 0.5] Adjusting the Spawn Rates of Enemy Types
  (`|ExecutionSequence`
    (:`then_0`
      (if (== (mod (`self.WaveCount`) 1) 0)
        (bind _result (`/Engine/EditorBlueprintResources/StandardMacros.IncrementInt` (`self.MaxArmoredCar_SpawnRateBase`))
          (:`  `
            (set `self.MaxArmoredCar_SpawnRateBase` _result)))))
    (:`then_1`
      (if (== (mod (`self.WaveCount`) 3) 0)
        (bind _result_2 (`/Engine/EditorBlueprintResources/StandardMacros.IncrementInt` (`self.MaxTank_SpawnRateBase`))
          (:`  `
            (set `self.MaxTank_SpawnRateBase` _result_2)))))
    (:`then_2`
      (if (== (mod (`self.WaveCount`) 7) 0)
        (bind _result_3 (`/Engine/EditorBlueprintResources/StandardMacros.IncrementInt` (`self.MaxAntiTank_SpawnRateBase`))
          (:`  `
            (set `self.MaxAntiTank_SpawnRateBase` _result_3)))))
    (:`then_3`
      (`self.E_WaveGameplayState`)
      (`self.MaxEnemySpawnCalculation`))))

(fn `E_WaveGameplayState`
  (bind _wavecount (`self.WaveCount`))
  (if (and (>= _wavecount 11) (<= _wavecount 20))
    (set `self.GameplayState` "NewEnumerator1")
    (set `self.EnemyMinSpawnDelay` 1.0)
    (set `self.EnemyMaxSpawnDelay` 2.0)
    (elif (>= (`self.WaveCount`) 21)
      (set `self.GameplayState` "NewEnumerator2")
      (set `self.EnemyMinSpawnDelay` 0.5)
      (set `self.EnemyMaxSpawnDelay` 1.0))))

(fn `GetSecondsToNextWave`
  (returns (Seconds :type "Float (double-precision)"))
  (return (+ (`self.WaveTimer`) (`KismetMathLibrary.Conv_IntToDouble` (`KismetMathLibrary.Clamp` (* (+ (`self.WaveCount`) 1) 5) 5 120)))))

(fn `MaxEnemySpawnCalculation`
  (bind _returnvalue (* (`self.WaveCount`) (`self.EnemySpawnModifier`)))
  (switch `/Game/TankGame/Ugurkan/BPs/Gameplay/E_WaveGameplayStatus` (`self.GameplayState`)
    (:`NewEnumerator0`
      (set `self.EnemySpawnModifier` 3)
      (set `self.MaxSpawnedEnemyValue` _returnvalue))
    (:`NewEnumerator1`
      (set `self.EnemySpawnModifier` 4)
      (set `self.MaxSpawnedEnemyValue` _returnvalue))
    (:`NewEnumerator2`
      (set `self.EnemySpawnModifier` 5)
      (set `self.MaxSpawnedEnemyValue` _returnvalue))))

(fn `PickEnemyType`
  (returns (EnemyType :type "/Game/TankGame/Ugurkan/BPs/Gameplay/EnemyInfos/E_EnemyTypes Enum") (RowName :type Name))
  (locals (Roll :type Integer :default 0))
  (bind _maxarmoredcar_spawnratebase (`self.MaxArmoredCar_SpawnRateBase`))
  (bind _roll (`local.Roll`))
  (bind _returnvalue (+ _maxarmoredcar_spawnratebase (`self.MaxTank_SpawnRateBase`)))
  (bind _returnvalue_2 (+ _returnvalue (`self.MaxAntiTank_SpawnRateBase`)))
  ; Weighted pick: roll 1..(sum of the three rates). Rates 3 / 1 / 0 = 75% car, 25% tank, no AT gun.
  ; Roll is kept in a local so it is rolled once (a pure Random node rolls again for every pin it feeds).
  (if (> _returnvalue_2 0)
    (set `local.Roll` (`KismetMathLibrary.RandomIntegerInRange` 1 _returnvalue_2))
    (if (<= _roll _maxarmoredcar_spawnratebase)
      (return "NewEnumerator1" "ArmoredCar_Row")
      (elif (<= _roll _returnvalue)
        (return "NewEnumerator0" "Tank_Row")
        (else
          (return "NewEnumerator2" "AntiTank_Row"))))
    (else
      (return "NewEnumerator0" "Tank_Row"))))

(fn `UserConstructionScript`)